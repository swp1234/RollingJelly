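; InGameController handles the touch-driven, one-shot aim and launch of the PlayingJelly player character.
; Pressing shows the DirectionViewer beam; dragging deprojects the touch to world space, setting the beam target and an X/Z launch direction from the starting position.
; Releasing hides the beam and launches the character along that direction, scaled by LaunchPower.
; Each tick, a character at or below the lower Z limit is teleported to that floor height at zero X/Y.
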(event `InputTouch`
  (params (Location :type "Vector Structure") (FingerIndex :type "ETouchIndex Enum"))
  (bind _worldposition (`GameplayStatics.DeprojectScreenToWorld` (`GameplayStatics.GetPlayerController` 0) (`KismetMathLibrary.Conv_VectorToVector2D` Location)))
  (bind (_returnvalue_x _returnvalue_y _returnvalue_z) (`KismetMathLibrary.BreakVector` (- _worldposition (`self.BasePoint`))))
  (bind _x (.x _worldposition))
  (bind _z (.z _worldposition))
  (:`Pressed`
    (if (not (`self.IsLaunched`))
      (set `self.IsReady` true)
      (bind _asplaying_jelly (cast `/Game/Blueprints/PlayingJelly` (`GameplayStatics.GetPlayerCharacter` 0)))
      (`SceneComponent.SetVisibility` (`/Game/Blueprints/PlayingJelly.DirectionViewer` _asplaying_jelly) true false)))
  (:`Released`
    (if (`self.IsReady`)
      (set `self.IsLaunched` true)
      (set `self.IsReady` false)
      (`Character.LaunchCharacter` (`GameplayStatics.GetPlayerCharacter` 0) (* (`self.LaunchDirection`) (`self.LaunchPower`)) true true)
      (bind _asplaying_jelly_2 (cast `/Game/Blueprints/PlayingJelly` (`GameplayStatics.GetPlayerCharacter` 0)))
      (`SceneComponent.SetVisibility` (`/Game/Blueprints/PlayingJelly.DirectionViewer` _asplaying_jelly_2) false false)))
  (:`Moved`
    (if (`self.IsReady`)
      (set `self.TouchingPoint` (`KismetMathLibrary.MakeVector` _x 0.0 _z))
      (set `self.LaunchDirection` (`KismetMathLibrary.Normal` (`KismetMathLibrary.MakeVector` _returnvalue_x 0.0 _returnvalue_z)))
      (bind _asplaying_jelly_3 (cast `/Game/Blueprints/PlayingJelly` (`GameplayStatics.GetPlayerCharacter` 0)))
      (`ParticleSystemComponent.SetBeamTargetPoint` (`/Game/Blueprints/PlayingJelly.DirectionViewer` _asplaying_jelly_3) 0 (`KismetMathLibrary.MakeVector` _x 0.0 _z) 0))))

(event `self.ReceiveBeginPlay`
  (set `self.IsLaunched` false)
  (set `self.BasePoint` (`SceneComponent.K2_GetComponentLocation` (`Actor.RootComponent` (`GameplayStatics.GetPlayerCharacter` 0)))))

(event `self.ReceiveTick`
  (params (DeltaSeconds :type "Float (single-precision)"))
  (`self.LimitActorZ`))

(fn `LimitActorZ`
  (bind (_returnvalue_x _returnvalue_y _returnvalue_z) (`KismetMathLibrary.BreakVector` (`SceneComponent.K2_GetComponentLocation` (`Actor.RootComponent` (`GameplayStatics.GetPlayerCharacter` 0)))))
  (if (<= _returnvalue_z -2000.0)
    (`self.K2_SetActorLocation` (`GameplayStatics.GetPlayerCharacter` 0) (0.0 0.0 -2000.0) false true)))

(fn `UserConstructionScript`)