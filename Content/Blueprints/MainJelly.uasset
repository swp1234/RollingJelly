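; MainJelly is a jelly character whose visual is a JellyWidget hosted in the JellyCharacter widget component.
; Its Turn function casts that component's widget to JellyWidget and forwards the TurnRight direction to it.
; Tick and BeginPlay are empty.
; A disconnected leftover chain would update animation and flip controller yaw by horizontal velocity, using MovingRight when stationary, but it never runs.
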(event `self.ReceiveTick`
  (params (DeltaSeconds :type "Float (single-precision)")))

(event `self.ReceiveBeginPlay`)

(fn `Turn`
  (params (TurnRight :type Boolean))
  (bind _asjelly_widget (cast `/Game/UI/Widget/JellyWidget` (`WidgetComponent.GetUserWidgetObject` (`self.JellyCharacter`))))
  (`/Game/UI/Widget/JellyWidget.Turn` _asjelly_widget TurnRight))

(fn `UserConstructionScript`)