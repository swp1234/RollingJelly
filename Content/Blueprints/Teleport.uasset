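; Teleporter actor that moves the player character to another actor tagged "Teleport" when the player overlaps its box.
; The overlap searches tagged actors other than itself, then calls a Teleport event that breaks the loop and is followed by a bubbling sound.
; The destination keeps the player's height relative to the teleporter, pins Y to a constant, and offsets X toward world zero, presumably to avoid retriggering.
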(event `self.Box.OnComponentBeginOverlap`
  (params (OverlappedComponent :type "PrimitiveComponent Object Reference") (OtherActor :type "Actor Object Reference") (OtherComp :type "PrimitiveComponent Object Reference") (OtherBodyIndex :type Integer) (bFromSweep :type Boolean) (SweepResult :type "HitResult Structure (by ref)"))
  (bind (_returnvalue_x _returnvalue_y _returnvalue_z) (`KismetMathLibrary.BreakVector` (- (`self.K2_GetActorLocation`) (`self.K2_GetActorLocation` (`GameplayStatics.GetPlayerCharacter` 0)))))
  (if (== OtherActor (`GameplayStatics.GetPlayerCharacter` 0))
    (bind _outactors (`GameplayStatics.GetAllActorsWithTag` "Teleport"))
    (for _array_element _outactors :!label _label
      (if (!= _array_element self)
        (`self.Teleport` (`self.K2_GetActorLocation` _array_element) _returnvalue_z)
        (`GameplayStatics.PlaySound2D` "/Game/Audio/teleport_bubbling.teleport_bubbling" 1.0 0.5 0.0 null null)))))

(event `Teleport`
  (params (TeleportLoc :type "Vector Structure") (Teleport_ZDistance :type "Float (double-precision)"))
  (`self.K2_SetActorLocation` (`GameplayStatics.GetPlayerCharacter` 0) (`KismetMathLibrary.MakeVector` (+ TeleportLoc_X (* (`self.Teleport_XOffset`) (select `bool` (< TeleportLoc_X 0.0) :`false` -1.0 :`true` 1.0 :!type "Float (single-precision)"))) 1.0 (- TeleportLoc_Z Teleport_ZDistance)) false false)
  (goto _label :!via `Break`))

(fn `UserConstructionScript`)